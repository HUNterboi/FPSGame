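; First-person player character Blueprint with movement, look, a crosshair widget and a hitscan rifle.
; Left mouse shows the muzzle particle and plays the AK sound through DoOnce gates, then hides, fades and resets them on release.
; Each press fires one camera line trace; a hit Ue4ASP_Character gets its mesh set to simulate physics and a fixed impulse on the hit bone.
; Movement follows the camera's forward and right vectors.
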(event `Key|LeftMouseButton`
  (params (Key :type "Key Structure"))
  (bind _camera (`self.Camera`))
  (bind _returnvalue (`SceneComponent.K2_GetComponentLocation` _camera))
  (:`Pressed`
    (`|ExecutionSequence`
      (:`then_0`
        ;[1 1 1] ShootingParticleView
        (`/Engine/EditorBlueprintResources/StandardMacros.DoOnce` false :!label _label
          (:`Completed`
            (`SceneComponent.SetVisibility` (`self.ShootingParticle`) true false))))
      (:`then_1`
        ;[1 1 1] ShootingSound
        (`/Engine/EditorBlueprintResources/StandardMacros.DoOnce` false :!label _label_2
          (:`Completed`
            (`AudioComponent.Play` (`self.AKSound`) 0.0))))
      (:`then_2`
        ;[1 1 1] Shoot
        (bind _outhit (`KismetSystemLibrary.LineTraceSingle` _returnvalue (+ _returnvalue (* (`SceneComponent.GetForwardVector` _camera) (`self.weaponRange`))) "TraceTypeQuery1" true))
        (bind (_bblockinghit _binitialoverlap _time _distance _location _impactpoint _normal _impactnormal _physmat _hitactor _hitcomponent _hitbonename) (`GameplayStatics.BreakHitResult` _outhit))
        (bind _asue_4asp_character (cast `/Game/AnimStarterPack/Ue4ASP_Character` _hitactor))
        (`|ExecutionSequence`
          (:`then_0`
            (bind _mesh (`Character.Mesh` _asue_4asp_character))
            (`PrimitiveComponent.SetSimulatePhysics` _mesh true)
            (`PrimitiveComponent.AddImpulse` _mesh (2000.0 2000.0 0.0) _hitbonename true))
          (:`then_1`
            (`KismetSystemLibrary.PrintString` "ENEMY SHOT"))))))
  (:`Released`
    (`|ExecutionSequence`
      (:`then_0`
        (`SceneComponent.SetVisibility` (`self.ShootingParticle`) false false)
        (goto _label :!via `Reset`))
      (:`then_1`
        (`AudioComponent.FadeOut` (`self.AKSound`) 0.3 0.0 "SCurve")
        (goto _label_2 :!via `Reset`)))))

(event `InputAxis|LookUp`
  (params (AxisValue :type "Float (single-precision)"))
  ;[1 1 1] camera
  (`self.AddControllerPitchInput` (`KismetMathLibrary.FClamp` AxisValue -1.0)))

(event `InputAxis|MoveRight`
  (params (AxisValue :type "Float (single-precision)"))
  ;[1 1 1] Movement
  (`self.AddMovementInput` (`SceneComponent.GetRightVector` (`self.Camera`)) AxisValue))

(event `InputAxis|MoveForward`
  (params (AxisValue :type "Float (single-precision)"))
  ;[1 1 1] Movement
  (`self.AddMovementInput` (`SceneComponent.GetForwardVector` (`self.Camera`)) AxisValue))

(event `InputAxis|LookRight`
  (params (AxisValue :type "Float (single-precision)"))
  ;[1 1 1] camera
  (`self.AddControllerYawInput` (`KismetMathLibrary.FClamp` AxisValue -1.0)))

(event `self.ReceiveBeginPlay`
  (`|ExecutionSequence`
    (:`then_0`
      ;[1 1 1] CrossHair
      (bind _returnvalue (`|CreateWidget` "/Game/UI/Crosshair.Crosshair_C" (`GameplayStatics.GetPlayerController` 0)))
      (`UserWidget.AddToViewport` _returnvalue 0))
    (:`then_1`
      ;[1 1 1] Do not shoot at start
      (`AudioComponent.Stop` (`self.AKSound`)))
    (:`then_2`
      (`SceneComponent.SetVisibility` (`self.ShootingParticle`) false false))))

(fn `UserConstructionScript`)